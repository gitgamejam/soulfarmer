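; Battle actor that runs an automatic one-on-one fight between the main character and a monster.
; On BeginPlay it spawns both at fixed, facing transforms and passes each a reference to the other.
; A looping fast timer makes both call Attack as long as either is alive, so attacks stop only when both are dead; the timer itself is never cleared.
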(event Custom|EnemyPlayerAttackEachOther
  ;[1 1 1] while battle is not finished, attack
  (if (or (not (Variables|/Game/SoulFarmer/Blueprints/MainCharacter_BP.MainCharacter_BP_C|GetisDead? (Variables|Default|GetPlayer))) (not (Variables|/Game/SoulFarmer/Blueprints/Monster_BP.Monster_BP_C|GetisDead? (Variables|Default|GetEnemy))))
    (Default|Attack (Variables|Default|GetPlayer))
    (Default|Attack (Variables|Default|GetEnemy))))

(event EventBeginPlay
  ;[1 1 1] Spawn and set Player
  (bind _returnvalue (Game|SpawnActorfromClass "/Game/SoulFarmer/Blueprints/MainCharacter_BP.MainCharacter_BP_C" (Math|Transform|MakeTransform "1229.997437,180.000000,206.001602" "0,-90.000000, 0") "Undefined" 0 0))
  (Variables|Default|SetPlayer _returnvalue)
  ;[1 1 1] Spawn and Set Enemy
  (bind _returnvalue_2 (Game|SpawnActorfromClass "/Game/SoulFarmer/Blueprints/Monster_BP.Monster_BP_C" (Math|Transform|MakeTransform "1229.997437,10.000000,206.001602" "0,90.000000,0.000000" "1.000000,1,1") "Undefined" 0 0))
  (Variables|Default|SetEnemy _returnvalue_2)
  ;[1 1 1] Set Enemy in player BP
  (Default|GetEnemy (Variables|Default|GetPlayer) (Variables|Default|GetEnemy))
  ;[1 1 1] Set Player in Enemy BP
  (Default|GetPlayer (Variables|Default|GetEnemy) (Variables|Default|GetPlayer))
  ;[1 1 1] while battle is not finished, attack
  (Utilities|Time|SetTimerbyEvent (delegate Custom|EnemyPlayerAttackEachOther) 0.05 true))

(event Collision|EventActorBeginOverlap
  (params (OtherActor :type Actor%20Object%20Reference)))

(event EventTick
  (params (DeltaSeconds :type Float%20%28single-precision%29)))

(fn ConstructionScript)