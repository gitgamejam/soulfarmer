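; Monster Blueprint for an enemy that fights the player in battles, with its own stats, delayed attacks and death flag.
; Construction script derives max HP from vitality and, for one class, damage from strength.
; A battle Blueprint assigns the player; Attack waits on attack speed, subtracts damage from the player's HP and calls its TakeDamage.
; TakeDamage only flags death at zero HP, so attackers apply the damage themselves.
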(event Custom|Calculate%20Stats
  (Utilities|FlowControl|Sequence
    (:then_0
      ;[1 1 1] calculate Max H
      (Variables|Stat|Setstat_maxHP (+ (Variables|Stat|Getstat_baseHP) (Variables|Attribute|Getatt_vitality)))
      ;[1 1 1] (get from stored date later)
      (Variables|Stat|Setstat_HP (Variables|Stat|Getstat_maxHP))
      ;[1 1 1] Calculate Base Damage
      (if (Utilities|Enum|Equal(Enum) (Variables|Default|GetClass) "NewEnumerator0")
        (Variables|Default|Setstat_damage (+ (Variables|Stat|Getstat_basedamage) (Variables|Attribute|Getatt_strength)))))))

(event Custom|Take%20Damage
  ;[1 1 1] If Hp below 0. Kill the actor
  (if (<= (Variables|Stat|Getstat_HP) 0)
    (Variables|Default|SetisDead? true)
    (Development|PrintString "monster is dead")))

(event Custom|Attack
  ;[1 1 1] Is the character dead?
  (if (not (Variables|Default|GetisDead?))
    ;[1 1 1] Attack
    (bind _asmain_character_bp (Utilities|Casting|CastToMainCharacter_BP (Variables|Default|GetPlayer)))
    ;[1 1 1] Is enemy dead?
    (if (not (Variables|/Game/SoulFarmer/Blueprints/MainCharacter_BP.MainCharacter_BP_C|GetisDead? _asmain_character_bp))
      (Utilities|FlowControl|Delay (Variables|Stat|Getstat_attackspeed))
      (bind _output_get (Variables|/Game/SoulFarmer/Blueprints/MainCharacter_BP.MainCharacter_BP_C|Setstat_HP _asmain_character_bp (- (Variables|/Game/SoulFarmer/Blueprints/MainCharacter_BP.MainCharacter_BP_C|Getstat_HP _asmain_character_bp) (Variables|Default|Getstat_damage))))
      ;[1 1 1] Notify the player take damage
      (Default|TakeDamage _asmain_character_bp)
      (Development|PrintString (Utilities|String|Append "Player HP: " (Utilities|String|ToString(Integer) _output_get))))))

(event Custom|Get%20Player
  (params (Player :type Actor%20Object%20Reference))
  ;[1 1 1] Set The Enemy - Assigned by Battle BP
  (Variables|Default|SetPlayer Player))

(event EventBeginPlay)

(event Collision|EventActorBeginOverlap
  (params (OtherActor :type Actor%20Object%20Reference)))

(event EventTick
  (params (DeltaSeconds :type Float%20%28single-precision%29)))

(fn ConstructionScript
  (|CallParentFunction)
  (CallFunction|CalculateStats))