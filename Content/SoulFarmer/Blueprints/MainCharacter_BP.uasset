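; MainCharacter_BP is the player character in SoulFarmer, holding combat stats and exchanging damage with a Monster_BP enemy assigned by the Battle BP.
; The construction script runs CalculateStats, deriving max HP from vitality and, for one class only, damage from strength.
; Each Attack call checks both are alive, waits the attack-speed delay, subtracts monster HP directly, then calls its TakeDamage.
; The character's own TakeDamage only flags death once HP runs out.
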(event Custom|Calculate%20Stats
  (Utilities|FlowControl|Sequence
    (:then_0
      ;[1 1 1] calculate Max H
      (Variables|Stat|Setstat_maxHP (+ (Variables|Stat|Getstat_baseHP) (Variables|Attribute|Getatt_vitality)))
      ;[1 1 1] (get from stored date later)
      (Variables|Stat|Setstat_HP (Variables|Stat|Getstat_maxHP))
      ;[1 1 1] Calculate Base Damage
      (if (Utilities|Enum|Equal(Enum) (Variables|Default|GetClass) "NewEnumerator0")
        (Variables|Default|Setstat_damage (+ (Variables|Stat|Getstat_basedamage) (Variables|Attribute|Getatt_strength)))))))

(event Custom|Take%20Damage
  ;[1 1 1] If Hp below 0. Kill the actor
  (if (<= (Variables|Stat|Getstat_HP) 0)
    (Variables|Default|SetisDead? true)
    (Development|PrintString "player is dead")))

(event Custom|Attack
  ;[1 1 1] Is the character dead?
  (if (not (Variables|Default|GetisDead?))
    ;[1 1 1] Attack
    (bind _asmonster_bp (Utilities|Casting|CastToMonster_BP (Variables|Default|GetEnemy)))
    ;[1 1 1] Is enemy dead?
    (if (not (Variables|/Game/SoulFarmer/Blueprints/Monster_BP.Monster_BP_C|GetisDead? _asmonster_bp))
      (bind _asmonster_bp_2 (Utilities|Casting|CastToMonster_BP (Variables|Default|GetEnemy)))
      (Utilities|FlowControl|Delay (Variables|Stat|Getstat_attackspeed))
      (bind _output_get (Variables|/Game/SoulFarmer/Blueprints/Monster_BP.Monster_BP_C|Setstat_HP _asmonster_bp_2 (- (Variables|/Game/SoulFarmer/Blueprints/Monster_BP.Monster_BP_C|Getstat_HP _asmonster_bp_2) (Variables|Default|Getstat_damage))))
      ;[1 1 1] Notify monster it take damage
      (Default|TakeDamage _asmonster_bp_2)
      (Development|PrintString (Utilities|String|Append "Monster HP: " (Utilities|String|ToString(Integer) _output_get))))))

(event Custom|Get%20Enemy
  (params (Enemy :type Actor%20Object%20Reference))
  ;[1 1 1] Set The Enemy - Assigned by Battle BP
  (Variables|Default|SetEnemy Enemy))

(event EventBeginPlay)

(event Collision|EventActorBeginOverlap
  (params (OtherActor :type Actor%20Object%20Reference)))

(event EventTick
  (params (DeltaSeconds :type Float%20%28single-precision%29)))

(fn ConstructionScript
  (|CallParentFunction)
  (CallFunction|CalculateStats))